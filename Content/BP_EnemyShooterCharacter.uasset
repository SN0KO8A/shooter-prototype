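; BP_EnemyShooterCharacter is an enemy shooter character with an overhead health bar and damage number feedback.
; On BeginPlay it hands itself to the WBP_Enemy_HealthBar widget as its ShooterOwner.
; Each tick it billboards the HPBar component toward the player camera manager's location.
; Any damage taken spawns a BP_DamageAmount actor at its transform, carrying the truncated damage value.
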(event `self.ReceiveBeginPlay`
  (`parent.ReceiveBeginPlay`)
  (bind _aswbp_enemy_health_bar (cast `/Game/UI/WBP_Enemy_HealthBar` (`WidgetComponent.GetUserWidgetObject` (`self.HP_Bar`))))
  (set `/Game/UI/WBP_Enemy_HealthBar.ShooterOwner` self _aswbp_enemy_health_bar))

(event `self.ReceiveTick`
  (params (DeltaSeconds :type "Float (single-precision)"))
  (bind _hp_bar (`self.HP_Bar`))
  (`parent.ReceiveTick` DeltaSeconds)
  (`SceneComponent.K2_SetWorldRotation` _hp_bar (`KismetMathLibrary.FindLookAtRotation` (`SceneComponent.K2_GetComponentLocation` _hp_bar) (`SceneComponent.K2_GetComponentLocation` (`PlayerCameraManager.TransformComponent` (`GameplayStatics.GetPlayerCameraManager` 0)))) false false))

(event `self.ReceiveAnyDamage`
  (params (Damage :type "Float (single-precision)") (DamageType :type "DamageType Object Reference") (InstigatedBy :type "Controller Object Reference") (DamageCauser :type "Actor Object Reference"))
  (`|SpawnActorFromClass` "/Game/BP_DamageAmount.BP_DamageAmount_C" (`self.GetTransform`) "Undefined" "MultiplyWithRoot" null (`KismetMathLibrary.FTrunc` Damage) null))

(fn `UserConstructionScript`
  (`parent.UserConstructionScript`))