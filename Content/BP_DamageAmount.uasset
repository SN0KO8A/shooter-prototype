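; BP_DamageAmount is a short-lived actor that shows a floating damage number.
; On BeginPlay it passes DamageAmount to the WBP_DamageText widget in its WBDamageAmount component, stopping early if the cast fails.
; MoveTimeline then lerps the actor from its spawn location along a fixed world-space offset, sideways and upward.
; The actor destroys itself when the timeline finishes.
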(event `self.ReceiveBeginPlay`
  (bind _aswbp_damage_text (cast `/Game/UI/WBP_DamageText` (`WidgetComponent.GetUserWidgetObject` (`self.WB_DamageAmount`))))
  (`/Game/UI/WBP_DamageText.SetDamage` _aswbp_damage_text (`self.Damage Amount`))
  (bind _output_get (set `self.StartLocation` (`self.K2_GetActorLocation`)))
  (set `self.EndLocation` (+ _output_get (-150.0 -150.0 50.0)))
  (bind (_direction _movetrack) (`Timeline|MoveTimeline`)
    (:`Update`
      (`self.K2_SetActorLocation` (`KismetMathLibrary.VLerp` (`self.StartLocation`) (`self.EndLocation`) _movetrack)))
    (:`Finished`
      (`self.K2_DestroyActor`))))

(fn `UserConstructionScript`)